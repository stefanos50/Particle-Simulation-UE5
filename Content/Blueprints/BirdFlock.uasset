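; Bird flock manager that spawns Particle_Boid actors in a box, shows the BirdFlockUI widget and makes itself the view target.
; A looping timer runs a boids simulation, summing separation, alignment and cohesion forces weighted by Multipliers through brute-force neighbor scans.
; Euler integration updates velocity and location, then moves and orients each skeletal mesh, with optional debug arrows.
; Steering clamps each axis between zero and MaxForce, discarding negative components.
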(event `AddParticle`
  (bind _box (`self.Box`))
  (bind _returnvalue (`KismetMathLibrary.RandomPointInBoundingBox` (`SceneComponent.K2_GetComponentLocation` _box) (`BoxComponent.BoxExtent` _box)))
  (bind _returnvalue_2 (`|SpawnActorFromClass` "/Game/Blueprints/Particle_Boid.Particle_Boid_C" (`KismetMathLibrary.MakeTransform` _returnvalue (struct) (0.5 0.5 0.5)) "Undefined" "OverrideRootScale" null null))
  (`KismetArrayLibrary.Array_Add` (`self.Boids`) _returnvalue_2)
  (set `/Game/Blueprints/Particle_Boid.Velocity` (`KismetMathLibrary.MakeVector` (`KismetMathLibrary.RandomFloatInRange` -10.0) (`KismetMathLibrary.RandomFloatInRange` 10.0) (`KismetMathLibrary.RandomFloatInRange` -10.0 10.0)) _returnvalue_2)
  (set `/Game/Blueprints/Particle_Boid.Mass` (`self.ParticleMass`) _returnvalue_2)
  (set `/Game/Blueprints/Particle_Boid.Location` _returnvalue _returnvalue_2)
  (set `/Game/Blueprints/Particle_Boid.Lifespan` (`self.BoidLifespan`) _returnvalue_2))

(event `self.ReceiveBeginPlay`
  (for _ (range (+ (`self.NumberOfParticles`) 1))
    (`self.AddParticle`))
  (bind _returnvalue (`|CreateWidget` "/Game/Blueprints/BirdFlockUI.BirdFlockUI_C"))
  (`UserWidget.AddToViewport` _returnvalue 0)
  (`WidgetBlueprintLibrary.SetInputMode_GameAndUIEx` null _returnvalue "DoNotLock" false)
  (`PlayerController.SetViewTargetWithBlend` (`GameplayStatics.GetPlayerControllerFromID` 0) self 0.0 "VTBlend_Linear" 0.0 false)
  (`KismetSystemLibrary.K2_SetTimer` null "RunSimulation" 0.03 true))

(event `self.ReceiveTick`
  (params (DeltaSeconds :type "Float (single-precision)")))

(event `self.ReceiveActorBeginOverlap`
  (params (OtherActor :type "Actor Object Reference")))

(fn `Align`
  (params (CurrentBoid :type "/Game/Blueprints/Particle_Boid Object Reference"))
  (returns (SteerForce :type "Vector Structure"))
  (locals (neighborist :type "Float (double-precision)" :default 200.0) (`location sum` :type "Vector Structure") (count :type Integer) (Steer :type "Vector Structure"))
  (bind _count (`local.count`))
  (bind _maxforce (`self.MaxForce`))
  (set `local.neighborist` (`self.NeighborDist`))
  (for _array_element (`self.Boids`)
    (`/Engine/EditorBlueprintResources/StandardMacros.IsValid` _array_element
      (:`Is Valid`
        (bind _returnvalue (`KismetMathLibrary.VSize` (- (`SceneComponent.K2_GetComponentLocation` (`/Game/Blueprints/Particle_Boid.SkeletalMesh` CurrentBoid)) (`SceneComponent.K2_GetComponentLocation` (`/Game/Blueprints/Particle_Boid.SkeletalMesh` _array_element)))))
        (if (and (> _returnvalue 0.0) (< _returnvalue (`local.neighborist`)))
          (set `local.location sum` (+ (`local.location sum`) (`/Game/Blueprints/Particle_Boid.Velocity` _array_element)))
          (`/Engine/EditorBlueprintResources/StandardMacros.IncrementInt` (`local.count`))))))
  (if (> _count 0)
    (bind _output_get (set `local.Steer` (* (`KismetMathLibrary.Normal` (/ (`local.location sum`) (`KismetMathLibrary.Conv_IntToDouble` _count))) (`self.MaxSpeed`))))
    (return (`KismetMathLibrary.MakeVector` (`KismetMathLibrary.FClamp` (.x _output_get) 0.0 _maxforce) (`KismetMathLibrary.FClamp` (.y _output_get) 0.0 _maxforce) (`KismetMathLibrary.FClamp` (.z _output_get) 0.0 _maxforce)))
    (else
      (bind _output_get_2 (set `local.Steer` (0.0 0.0 0.0)))
      (return _output_get_2))))

(fn `Cohesion`
  (params (CurrentBoid :type "/Game/Blueprints/Particle_Boid Object Reference") (CurrentBoidLocation :type "Vector Structure") (CurrentVelocity :type "Vector Structure"))
  (returns (SteerForce :type "Vector Structure"))
  (locals (neighborist :type "Float (double-precision)" :default 200.0) (sum :type "Vector Structure") (count :type Integer))
  (bind _count (`local.count`))
  (set `local.neighborist` (`self.NeighborDist`))
  (for _array_element (`self.Boids`)
    (`/Engine/EditorBlueprintResources/StandardMacros.IsValid` _array_element
      (:`Is Valid`
        (bind _returnvalue (`KismetMathLibrary.VSize` (- (`SceneComponent.K2_GetComponentLocation` (`/Game/Blueprints/Particle_Boid.SkeletalMesh` CurrentBoid)) (`SceneComponent.K2_GetComponentLocation` (`/Game/Blueprints/Particle_Boid.SkeletalMesh` _array_element)))))
        (if (and (> _returnvalue 0.0) (< _returnvalue (`local.neighborist`)))
          (set `local.sum` (+ (`/Game/Blueprints/Particle_Boid.Location` _array_element) (`local.sum`)))
          (`/Engine/EditorBlueprintResources/StandardMacros.IncrementInt` (`local.count`))))))
  (if (> _count 0)
    (bind _steerforce (`self.Seek` (/ (`local.sum`) _count) CurrentBoidLocation CurrentVelocity))
    (return _steerforce)
    (else
      (return (0.0 0.0 0.0)))))

(fn `DrawDebugDynamics`
  (params (Location :type "Vector Structure") (Velocity :type "Vector Structure") (Mass :type "Float (double-precision)") (Bforce :type "Vector Structure"))
  (if (`self.Debug?`)
    (`KismetSystemLibrary.DrawDebugArrow` Location (* (+ Location (* Velocity (* (`self.gravity`) Mass))) (1.0 1.0 2.0)) 25.0 (struct :`R` 1.0 :`B` 0.018362 :`A` 1.0) 0.001 5.0)
    (`KismetSystemLibrary.DrawDebugArrow` Location (+ Location (* Velocity (100.0 100.0 100.0))) 25.0 (struct :`R` 0.974049 :`G` 1.0 :`A` 1.0) 0.001 5.0)
    (`KismetSystemLibrary.DrawDebugArrow` Location (+ Location (+ Velocity (* Bforce (100.0 100.0 100.0)))) 25.0 (struct :`R` 0.09355 :`G` 0.817708 :`A` 1.0) 0.001 5.0)))

(fn `Euler`
  (params (Location :type "Vector Structure") (Velocity :type "Vector Structure") (time :type "Float (double-precision)") (Mass :type "Float (double-precision)") (FlockForce :type "Vector Structure"))
  (returns (NewLocation :type "Vector Structure") (NewVelocity :type "Vector Structure"))
  (return (+ Location (* Velocity (`KismetMathLibrary.MakeVector` time time time))) (+ Velocity (* (/ FlockForce (`KismetMathLibrary.MakeVector` Mass Mass Mass)) (`KismetMathLibrary.MakeVector` time time time)))))

(fn `Flock`
  (params (CurrentBoid :type "/Game/Blueprints/Particle_Boid Object Reference") (`Current Velocity` :type "Vector Structure") (`Current Position` :type "Vector Structure"))
  (returns (`Force Final` :type "Vector Structure"))
  (bind (_multipliers_x _multipliers_y _multipliers_z) (`KismetMathLibrary.BreakVector` (`self.Multipliers`)))
  (bind _steerforce (`self.Separate` CurrentBoid `Current Position`))
  (bind _steerforce_2 (`self.Align` CurrentBoid))
  (bind _steerforce_3 (`self.Cohesion` CurrentBoid `Current Position` `Current Velocity`))
  (return (+ (* _steerforce _multipliers_x) (* _steerforce_2 _multipliers_y) (* _steerforce_3 _multipliers_z))))

(fn `get_vector_float`
  (params (Vector1 :type "Vector Structure") (Vector2 :type "Vector Structure"))
  (returns (Result :type "Float (double-precision)"))
  (return (+ (* Vector1_X Vector2_X) (* Vector1_Y Vector2_Y) (* Vector1_Z Vector2_Z))))

(fn `RunSimulation`
  (bind _t0 (`self.t0`))
  (bind _boids (`self.Boids`))
  (for (_array_element _array_index) _boids
    (`/Engine/EditorBlueprintResources/StandardMacros.IsValid` _array_element
      (:`Is Valid`
        (bind _velocity (`/Game/Blueprints/Particle_Boid.Velocity` _array_element))
        (bind _location (`/Game/Blueprints/Particle_Boid.Location` _array_element))
        (bind _force_final (`self.Flock` _array_element _velocity _location))
        (bind _mass (`/Game/Blueprints/Particle_Boid.Mass` _array_element))
        (`self.DrawDebugDynamics` _location _velocity _mass _force_final)
        (set `/Game/Blueprints/Particle_Boid.Lifespan` (- (`/Game/Blueprints/Particle_Boid.Lifespan` _array_element) _t0) _array_element)
        (bind (_newlocation _newvelocity) (`self.Euler` _location _velocity (+ (`self.t`) _t0) _mass _force_final))
        (bind _output_get (set `/Game/Blueprints/Particle_Boid.Location` _newlocation _array_element))
        (set `/Game/Blueprints/Particle_Boid.Velocity` _newvelocity _array_element)
        (bind _skeletalmesh (`/Game/Blueprints/Particle_Boid.SkeletalMesh` _array_element))
        (`SceneComponent.K2_SetWorldLocation` _skeletalmesh _output_get true false)
        (`SceneComponent.K2_SetWorldRotation` _skeletalmesh (* (`KismetMathLibrary.FindLookAtRotation` _newlocation (+ _newlocation (* _newvelocity (100.0 100.0 100.0)))) -1.0) false false))
      (:`Is Not Valid`
        (`KismetArrayLibrary.Array_Remove` _boids _array_index)))))

(fn `Seek`
  (params (Target :type "Vector Structure") (position :type "Vector Structure") (velocity :type "Vector Structure"))
  (returns (SteerForce :type "Vector Structure"))
  (bind _maxforce (`self.MaxForce`))
  (bind (_returnvalue_x _returnvalue_y _returnvalue_z) (`KismetMathLibrary.BreakVector` (- (* (`KismetMathLibrary.Normal` (- Target position)) (`self.MaxSpeed`)) velocity)))
  (return (`KismetMathLibrary.MakeVector` (`KismetMathLibrary.FClamp` _returnvalue_x 0.0 _maxforce) (`KismetMathLibrary.FClamp` _returnvalue_y 0.0 _maxforce) (`KismetMathLibrary.FClamp` _returnvalue_z 0.0 _maxforce))))

(fn `Separate`
  (params (CurrentBoid :type "/Game/Blueprints/Particle_Boid Object Reference") (Velocity :type "Vector Structure"))
  (returns (SteerForce :type "Vector Structure"))
  (locals (desiredSeparation :type "Float (double-precision)" :default 100.0) (Steer :type "Vector Structure") (count :type Integer))
  (bind _steer (`local.Steer`))
  (bind _count (`local.count`))
  (bind _steer_2 (`local.Steer`))
  (bind _maxforce (`self.MaxForce`))
  (bind (_returnvalue_x _returnvalue_y _returnvalue_z) (`KismetMathLibrary.BreakVector` (- (* (`KismetMathLibrary.Normal` _steer_2) (`self.MaxSpeed`)) Velocity)))
  (set `local.desiredSeparation` (`self.SepatateDist`))
  (for _array_element (`self.Boids`)
    (`/Engine/EditorBlueprintResources/StandardMacros.IsValid` _array_element
      (:`Is Valid`
        (bind _returnvalue (- (`SceneComponent.K2_GetComponentLocation` (`/Game/Blueprints/Particle_Boid.SkeletalMesh` CurrentBoid)) (`SceneComponent.K2_GetComponentLocation` (`/Game/Blueprints/Particle_Boid.SkeletalMesh` _array_element))))
        (bind _returnvalue_2 (`KismetMathLibrary.VSize` _returnvalue))
        (if (and (> _returnvalue_2 0.0) (< _returnvalue_2 (`local.desiredSeparation`)))
          (set `local.Steer` (+ _steer (/ (`KismetMathLibrary.Normal` _returnvalue) _returnvalue_2)))
          (`/Engine/EditorBlueprintResources/StandardMacros.IncrementInt` _count)))))
  (if (> _count 0)
    (set `local.Steer` (/ _steer (`KismetMathLibrary.Conv_IntToDouble` _count))))
  (if (> (`KismetMathLibrary.VSize` _steer_2) 0.0)
    (bind _output_get (set `local.Steer` (`KismetMathLibrary.MakeVector` (`KismetMathLibrary.FClamp` _returnvalue_x 0.0 _maxforce) (`KismetMathLibrary.FClamp` _returnvalue_y 0.0 _maxforce) (`KismetMathLibrary.FClamp` _returnvalue_z 0.0 _maxforce))))
    (return _output_get)
    (else
      (return (`local.Steer`)))))

(fn `UserConstructionScript`)