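; Fire particle simulator actor that spawns glowing red Particle_Ball actors at random points in a fixed area, takes the camera view and shows FireUI.
; Looping timers drive spawning, whose rate NewSpawnRate changes, and RunSimulation, which decrements lifespans and drops invalid particles.
; Each step moves particles by hand-written Euler integration of gravity and wind, without engine physics.
; A Debug flag draws per-particle velocity and force arrows.
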(event `AddParticle`
  (bind _returnvalue (`KismetMathLibrary.MakeVector` (`KismetMathLibrary.RandomFloatInRange` -199.414213 159.764495) (`KismetMathLibrary.RandomFloatInRange` 193.260653 -209.627013) 749.999995))
  (bind _returnvalue_2 (`|SpawnActorFromClass` "/Game/Blueprints/Particle_Ball.Particle_Ball_C" (`KismetMathLibrary.MakeTransform` _returnvalue) "Undefined" "OverrideRootScale" null null))
  (`KismetArrayLibrary.Array_Add` (`self.ActiveParticles`) _returnvalue_2)
  (set `/Game/Blueprints/Particle_Ball.Velocity` (`KismetMathLibrary.MakeVector` (`KismetMathLibrary.RandomFloatInRange` 0.0) (`KismetMathLibrary.RandomFloatInRange` 0.0) (`KismetMathLibrary.RandomFloatInRange` 1.0 2.0)) _returnvalue_2)
  (set `/Game/Blueprints/Particle_Ball.Mass` (`self.ParticleMass`) _returnvalue_2)
  (set `/Game/Blueprints/Particle_Ball.Location` _returnvalue _returnvalue_2)
  (set `/Game/Blueprints/Particle_Ball.Lifespan` (`KismetMathLibrary.RandomFloatInRange` 5.0 120.0) _returnvalue_2)
  (bind _returnvalue_3 (`PrimitiveComponent.CreateDynamicMaterialInstance` (`/Game/Blueprints/Particle_Ball.Sphere` _returnvalue_2) 0 "/Game/Colors/ColorMaterial_Inst.ColorMaterial_Inst" "None"))
  (`MaterialInstanceDynamic.SetVectorParameterValue` _returnvalue_3 "Color" (struct :`R` 1.0 :`A` 1.0))
  (`MaterialInstanceDynamic.SetScalarParameterValue` _returnvalue_3 "Intensity" 20.0)
  (set `/Game/Blueprints/Particle_Ball.ColorMaterial` _returnvalue_3 _returnvalue_2))

(event `ParticlesInit`
  (for _ (range (+ (`self.NumberOfParticles`) 1))
    (`self.AddParticle`)))

(event `self.ReceiveBeginPlay`
  (`self.ParticlesInit`)
  (`KismetSystemLibrary.K2_SetTimer` null "RunSimulation" 0.01 true)
  (bind _returnvalue (`KismetSystemLibrary.K2_SetTimer` null "SpawnNewParticle" 0.004 true))
  (set `self.SpawnTimer` _returnvalue)
  (`PlayerController.SetViewTargetWithBlend` (`GameplayStatics.GetPlayerControllerFromID` 0) self 0.0 "VTBlend_Linear" 0.0 false)
  (bind _returnvalue_2 (`|CreateWidget` "/Game/Blueprints/FireUI.FireUI_C"))
  (`UserWidget.AddToViewport` _returnvalue_2 0)
  (`WidgetBlueprintLibrary.SetInputMode_GameAndUIEx` (`GameplayStatics.GetPlayerController` 0) _returnvalue_2))

(event `self.ReceiveTick`
  (params (DeltaSeconds :type "Float (single-precision)")))

(event `NewSpawnRate`
  (params (Rate :type "Float (double-precision)"))
  (`KismetSystemLibrary.K2_InvalidateTimerHandle` (`self.SpawnTimer`))
  (`KismetSystemLibrary.K2_SetTimer` null "SpawnNewParticle" Rate true))

(fn `DrawDebugDynamics`
  (params (Location :type "Vector Structure") (Velocity :type "Vector Structure") (Mass :type "Float (double-precision)"))
  (if (`self.Debug?`)
    (`KismetSystemLibrary.DrawDebugArrow` Location (* (+ Location (* Velocity (* (`self.gravity`) Mass))) (1.0 1.0 1.1)) 25.0 (struct :`R` 1.0 :`B` 0.018362 :`A` 1.0) 0.001 5.0)
    (`KismetSystemLibrary.DrawDebugArrow` Location (+ Location (* Velocity (50.0 50.0 50.0))) 25.0 (struct :`R` 0.974049 :`G` 1.0 :`A` 1.0) 0.001 5.0)
    (`KismetSystemLibrary.DrawDebugArrow` Location (+ Location (* (* (`self.WindVelocity`) (500.0 500.0 500.0)) (`self.kv`))) 25.0 (struct :`R` 0.09355 :`G` 0.817708 :`A` 1.0) 0.001 5.0)))

(fn `Euler`
  (params (Location :type "Vector Structure") (Velocity :type "Vector Structure") (time :type "Float (double-precision)") (Mass :type "Float (double-precision)"))
  (returns (NewLocation :type "Vector Structure") (NewVelocity :type "Vector Structure"))
  (return (+ Location (* Velocity (`KismetMathLibrary.MakeVector` time time time))) (+ Velocity (* (/ (+ (* (`self.gravity`) Mass) (* (`self.kv`) (`self.WindVelocity`))) (`KismetMathLibrary.MakeVector` Mass Mass Mass)) (`KismetMathLibrary.MakeVector` time time time)))))

(fn `get_vector_float`
  (params (Vector1 :type "Vector Structure") (Vector2 :type "Vector Structure"))
  (returns (Result :type "Float (double-precision)"))
  (return (+ (* Vector1_X Vector2_X) (* Vector1_Y Vector2_Y) (* Vector1_Z Vector2_Z))))

(fn `RunSimulation`
  (bind _t0 (`self.t0`))
  (bind _activeparticles (`self.ActiveParticles`))
  (for (_array_element _array_index) _activeparticles
    (`/Engine/EditorBlueprintResources/StandardMacros.IsValid` _array_element
      (:`Is Valid`
        (bind _output_get (set `/Game/Blueprints/Particle_Ball.Lifespan` (- (`/Game/Blueprints/Particle_Ball.Lifespan` _array_element) _t0) _array_element))
        (bind _location (`/Game/Blueprints/Particle_Ball.Location` _array_element))
        (bind _velocity (`/Game/Blueprints/Particle_Ball.Velocity` _array_element))
        (bind _mass (`/Game/Blueprints/Particle_Ball.Mass` _array_element))
        (`self.DrawDebugDynamics` _location _velocity _mass)
        (bind (_newlocation _newvelocity) (`self.Euler` _location _velocity (+ (`self.t`) _t0) _mass))
        (bind _output_get_2 (set `/Game/Blueprints/Particle_Ball.Location` _newlocation _array_element))
        (set `/Game/Blueprints/Particle_Ball.Velocity` _newvelocity _array_element)
        (`SceneComponent.K2_SetWorldLocation` (`/Game/Blueprints/Particle_Ball.Sphere` _array_element) _output_get_2 false false))
      (:`Is Not Valid`
        (`KismetArrayLibrary.Array_Remove` _activeparticles _array_index)))))

(fn `SpawnNewParticle`
  (`self.AddParticle`))

(fn `UserConstructionScript`)