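; Particle simulation actor that spawns randomly coloured Particle_Ball actors inside a box, becomes the view target and shows the Simulation1UI widget.
; Timers keep adding balls and run RunSimulation, which ages them, prunes invalid entries and Euler-integrates gravity and a velocity-proportional force.
; CollisionDetector tests six axis-aligned planes by dot product; on a hit, the step re-integrates using the computed impact time and an Epsilon-adjusted velocity.
; Optional debug arrows visualise the dynamics.
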(event `AddParticle`
  (bind (_maxminvelocity_x _maxminvelocity_y _maxminvelocity_z) (`KismetMathLibrary.BreakVector` (`self.MaxMinVelocity`)))
  (bind _returnvalue (`SceneComponent.K2_GetComponentLocation` (`self.SpawnPoint`)))
  (bind _returnvalue_2 (`|SpawnActorFromClass` "/Game/Blueprints/Particle_Ball.Particle_Ball_C" (`KismetMathLibrary.MakeTransform` _returnvalue (struct) (0.3 0.3 0.3)) "Undefined" "OverrideRootScale" null null))
  (`KismetArrayLibrary.Array_Add` (`self.ActiveParticles`) _returnvalue_2)
  (set `/Game/Blueprints/Particle_Ball.Velocity` (`KismetMathLibrary.MakeVector` (`KismetMathLibrary.RandomFloatInRange` _maxminvelocity_y _maxminvelocity_x) (`KismetMathLibrary.RandomFloatInRange` _maxminvelocity_y _maxminvelocity_x) (`KismetMathLibrary.RandomFloatInRange` _maxminvelocity_z _maxminvelocity_x)) _returnvalue_2)
  (set `/Game/Blueprints/Particle_Ball.Mass` (`self.ParticleMass`) _returnvalue_2)
  (set `/Game/Blueprints/Particle_Ball.Location` _returnvalue _returnvalue_2)
  (set `/Game/Blueprints/Particle_Ball.Lifespan` (`self.particle_lifespan`) _returnvalue_2)
  (bind _returnvalue_3 (`PrimitiveComponent.CreateDynamicMaterialInstance` (`/Game/Blueprints/Particle_Ball.Sphere` _returnvalue_2) 0 "/Game/Colors/ColorMaterial_Inst.ColorMaterial_Inst" "None"))
  (`MaterialInstanceDynamic.SetVectorParameterValue` _returnvalue_3 "Color" (`KismetMathLibrary.MakeColor` (`KismetMathLibrary.RandomFloatInRange` 0.0 255.0) (`KismetMathLibrary.RandomFloatInRange` 0.0 255.0) (`KismetMathLibrary.RandomFloatInRange` 0.0 255.0)))
  (`MaterialInstanceDynamic.SetScalarParameterValue` _returnvalue_3 "Intensity" (`KismetMathLibrary.RandomFloatInRange` 0.1 0.2))
  (set `/Game/Blueprints/Particle_Ball.ColorMaterial` _returnvalue_3 _returnvalue_2))

(event `ParticlesInit`
  (for _ (range (+ (`self.NumberOfParticles`) 1))
    (`self.AddParticle`)))

(event `self.ReceiveBeginPlay`
  (`self.ParticlesInit`)
  (`KismetSystemLibrary.K2_SetTimer` null "RunSimulation" 0.01 true)
  (`KismetSystemLibrary.K2_SetTimerDelegate` (delegate `AddParticle`) 0.1 true)
  (`PlayerController.SetViewTargetWithBlend` (`GameplayStatics.GetPlayerControllerFromID` 0) self 0.0 "VTBlend_Linear" 0.0 false)
  (bind _returnvalue (`|CreateWidget` "/Game/Blueprints/Simulation1UI.Simulation1UI_C"))
  (`UserWidget.AddToViewport` _returnvalue 0)
  (`WidgetBlueprintLibrary.SetInputMode_GameAndUIEx` (`GameplayStatics.GetPlayerController` 0) _returnvalue "DoNotLock" false))

(event `self.ReceiveTick`
  (params (DeltaSeconds :type "Float (single-precision)")))

(fn `CalculateLastValidTime`
  (params (LastLocation :type "Vector Structure") (LastVelocity :type "Vector Structure") (PointName :type String) (ImpactPoint :type "Vector Structure") (NormalVector :type "Vector Structure"))
  (returns (NewT :type "Float (double-precision)") (Vnormal :type "Vector Structure"))
  (bind (_x _y _z) (`KismetMathLibrary.BreakVector3f` LastVelocity))
  (bind _returnvalue (* NormalVector (`KismetMathLibrary.MakeVector` -1.0 -1.0 -1.0)))
  (bind _returnvalue_2 (/ (- (.y ImpactPoint) (.y LastLocation)) _y))
  (bind _returnvalue_3 (/ (- (.x ImpactPoint) (.x LastLocation)) _x))
  (bind _returnvalue_4 (/ (- (.z ImpactPoint) (.z LastLocation)) _z))
  (switch `string` PointName
    (:`Point1`
      (return _returnvalue_3 _returnvalue))
    (:`Point2`
      (return _returnvalue_3 _returnvalue))
    (:`Point3`
      (return _returnvalue_2 _returnvalue))
    (:`Point4`
      (return _returnvalue_2 _returnvalue))
    (:`Point5`
      (return _returnvalue_4 _returnvalue))
    (:`Point6`
      (return _returnvalue_4 _returnvalue))))

(fn `Collision_Detector`
  (params (NewParticleLocation :type "Vector Structure"))
  (returns (`Collision?` :type Boolean) (NormalVector :type "Vector Structure") (PointName :type String) (PointLocation :type "Vector Structure"))
  (bind _returnvalue (`KismetMathLibrary.MakeVector` -1.0))
  (bind _returnvalue_2 (`KismetMathLibrary.MakeVector` 0.0 0.0 -1.0))
  (bind _returnvalue_3 (`KismetMathLibrary.MakeVector` 0.0 0.0 1.0))
  (bind _returnvalue_4 (`KismetMathLibrary.MakeVector` 0.0 1.0))
  (bind _returnvalue_5 (`KismetMathLibrary.MakeVector` 0.0 -1.0))
  (bind _returnvalue_6 (`KismetMathLibrary.MakeVector` 1.0))
  (bind _returnvalue_7 (`SceneComponent.K2_GetComponentLocation` (`self.Point4`)))
  (bind _returnvalue_8 (`SceneComponent.K2_GetComponentLocation` (`self.Point2`)))
  (bind _returnvalue_9 (`SceneComponent.K2_GetComponentLocation` (`self.Point6`)))
  (bind _returnvalue_10 (`SceneComponent.K2_GetComponentLocation` (`self.Point5`)))
  (bind _returnvalue_11 (`SceneComponent.K2_GetComponentLocation` (`self.Point3`)))
  (bind _returnvalue_12 (`SceneComponent.K2_GetComponentLocation` (`self.Point1`)))
  (bind _returnvalue_13 (< (`self.get_vector_float` _returnvalue_2 (- NewParticleLocation _returnvalue_9)) 0.0))
  (bind _returnvalue_14 (< (`self.get_vector_float` _returnvalue_3 (- NewParticleLocation _returnvalue_10)) 0.0))
  (bind _returnvalue_15 (< (`self.get_vector_float` _returnvalue_4 (- NewParticleLocation _returnvalue_11)) 0.0))
  (bind _returnvalue_16 (< (`self.get_vector_float` _returnvalue_5 (- NewParticleLocation _returnvalue_7)) 0.0))
  (bind _returnvalue_17 (< (`self.get_vector_float` _returnvalue_6 (- NewParticleLocation _returnvalue_12)) 0.0))
  (bind _returnvalue_18 (< (`self.get_vector_float` _returnvalue (- NewParticleLocation _returnvalue_8)) 0.0))
  (bind _returnvalue_19 (or _returnvalue_17 _returnvalue_18 _returnvalue_13 _returnvalue_14 _returnvalue_15 _returnvalue_16))
  (`|ExecutionSequence`
    (:`then_0`
      (if _returnvalue_17
        (return _returnvalue_19 _returnvalue_6 "Point1" _returnvalue_12)))
    (:`then_1`
      (if _returnvalue_18
        (return _returnvalue_19 _returnvalue "Point2" _returnvalue_8)))
    (:`then_2`
      (if _returnvalue_13
        (return _returnvalue_19 _returnvalue_2 "Point6" _returnvalue_9)))
    (:`then_3`
      (if _returnvalue_14
        (return _returnvalue_19 _returnvalue_3 "Point5" _returnvalue_10)))
    (:`then_4`
      (if _returnvalue_15
        (return _returnvalue_19 _returnvalue_4 "Point3" _returnvalue_11)))
    (:`then_5`
      (if _returnvalue_16
        (return _returnvalue_19 _returnvalue_5 "Point4" _returnvalue_7)))
    (:`then_6`
      (if (not _returnvalue_19)
        (return _returnvalue_19 (0.0 0.0 0.0) "None" (0.0 0.0 0.0))))))

(fn `DrawDebugDynamics`
  (params (Location :type "Vector Structure") (Velocity :type "Vector Structure") (Mass :type "Float (double-precision)"))
  (if (`self.Debug?`)
    (`KismetSystemLibrary.DrawDebugArrow` Location (* (+ Location (* Velocity (* (`self.gravity`) Mass))) (1.0 1.0 2.0)) 25.0 (struct :`R` 1.0 :`B` 0.018362 :`A` 1.0) 0.001 5.0)
    (`KismetSystemLibrary.DrawDebugArrow` Location (+ Location (* Velocity (100.0 100.0 100.0))) 25.0 (struct :`R` 0.974049 :`G` 1.0 :`A` 1.0) 0.001 5.0)
    (`KismetSystemLibrary.DrawDebugArrow` Location (+ Location (* (* Velocity (500.0 500.0 500.0)) (`self.kv`))) 25.0 (struct :`R` 0.09355 :`G` 0.817708 :`A` 1.0) 0.001 5.0)))

(fn `Euler`
  (params (Location :type "Vector Structure") (Velocity :type "Vector Structure") (time :type "Float (double-precision)") (Mass :type "Float (double-precision)"))
  (returns (NewLocation :type "Vector Structure") (NewVelocity :type "Vector Structure"))
  (bind _kv (`self.kv`))
  (return (+ Location (* Velocity (`KismetMathLibrary.MakeVector` time time time))) (+ Velocity (* (/ (+ (* (`self.gravity`) Mass) (* Velocity (`KismetMathLibrary.MakeVector` _kv _kv _kv))) (`KismetMathLibrary.MakeVector` Mass Mass Mass)) (`KismetMathLibrary.MakeVector` time time time)))))

(fn `get_vector_float`
  (params (Vector1 :type "Vector Structure") (Vector2 :type "Vector Structure"))
  (returns (Result :type "Float (double-precision)"))
  (return (+ (* Vector1_X Vector2_X) (* Vector1_Y Vector2_Y) (* Vector1_Z Vector2_Z))))

(fn `RunSimulation`
  (bind _t0 (`self.t0`))
  (bind _activeparticles (`self.ActiveParticles`))
  (bind _epsilon (`self.epsilon`))
  (for (_array_element _array_index) _activeparticles
    (`/Engine/EditorBlueprintResources/StandardMacros.IsValid` _array_element
      (:`Is Valid`
        (bind _location (`/Game/Blueprints/Particle_Ball.Location` _array_element))
        (bind _velocity (`/Game/Blueprints/Particle_Ball.Velocity` _array_element))
        (bind _mass (`/Game/Blueprints/Particle_Ball.Mass` _array_element))
        (`self.DrawDebugDynamics` _location _velocity _mass)
        (set `/Game/Blueprints/Particle_Ball.Lifespan` (- (`/Game/Blueprints/Particle_Ball.Lifespan` _array_element) _t0) _array_element)
        (bind (_newlocation _newvelocity) (`self.Euler` _location _velocity (+ (`self.t`) _t0) _mass))
        (bind (_collision_ _normalvector _pointname _pointlocation) (`self.Collision_Detector` _newlocation))
        (if _collision_
          (bind (_newt _vnormal) (`self.CalculateLastValidTime` _location _velocity _pointname _pointlocation _normalvector))
          (bind _newlocation_2 (`self.Euler` _location _velocity _newt _mass))
          (bind (_newlocation_3 _newvelocity_2) (`self.Euler` _newlocation_2 (+ (* (`KismetMathLibrary.MakeVector` _epsilon _epsilon _epsilon) _vnormal) (- _velocity _vnormal)) _newt _mass))
          (bind _output_get (set `/Game/Blueprints/Particle_Ball.Location` _newlocation_3 _array_element))
          (set `/Game/Blueprints/Particle_Ball.Velocity` _newvelocity_2 _array_element)
          (`SceneComponent.K2_SetWorldLocation` (`/Game/Blueprints/Particle_Ball.Sphere` _array_element) _output_get false false)
          (else
            (bind _output_get_2 (set `/Game/Blueprints/Particle_Ball.Location` _newlocation _array_element))
            (set `/Game/Blueprints/Particle_Ball.Velocity` _newvelocity _array_element)
            (`SceneComponent.K2_SetWorldLocation` (`/Game/Blueprints/Particle_Ball.Sphere` _array_element) _output_get_2 false false))))
      (:`Is Not Valid`
        (`KismetArrayLibrary.Array_Remove` _activeparticles _array_index)))))

(fn `UserConstructionScript`)