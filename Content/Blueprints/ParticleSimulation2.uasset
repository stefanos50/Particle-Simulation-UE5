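; Particle simulation actor that spawns randomly coloured balls with random velocities around a spherical boundary, takes over the view and shows the SphereSimUI widget.
; A looping timer runs RunSimulation, which sums pairwise inverse-square forces per particle and advances each by Euler integration.
; When a step lands outside the sphere, a quadratic solver finds the contact time and velocity is adjusted along the normal.
; Optional debug arrows show force and velocity.
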(event `AddParticle`
  (bind (_maxminvelocity_x _maxminvelocity_y _maxminvelocity_z) (`KismetMathLibrary.BreakVector` (`self.MaxMinVelocity`)))
  (bind _returnvalue (`SceneComponent.K2_GetComponentLocation` (`self.SpawnPoint`)))
  (bind _returnvalue_2 (`|SpawnActorFromClass` "/Game/Blueprints/Particle_Ball.Particle_Ball_C" (`KismetMathLibrary.MakeTransform` _returnvalue (struct) (0.3 0.3 0.3)) "Undefined" "OverrideRootScale" null null))
  (`KismetArrayLibrary.Array_Add` (`self.ActiveParticles`) _returnvalue_2)
  (set `/Game/Blueprints/Particle_Ball.Velocity` (`KismetMathLibrary.MakeVector` (`KismetMathLibrary.RandomFloatInRange` _maxminvelocity_x _maxminvelocity_y) (`KismetMathLibrary.RandomFloatInRange` _maxminvelocity_x _maxminvelocity_y) (`KismetMathLibrary.RandomFloatInRange` _maxminvelocity_z _maxminvelocity_y)) _returnvalue_2)
  (set `/Game/Blueprints/Particle_Ball.Mass` (`self.ParticleMass`) _returnvalue_2)
  (set `/Game/Blueprints/Particle_Ball.Location` (`KismetMathLibrary.MakeVector` (.x _returnvalue) (.y _returnvalue) (.z _returnvalue)) _returnvalue_2)
  (set `/Game/Blueprints/Particle_Ball.Lifespan` (`self.particle_lifespan`) _returnvalue_2)
  (bind _returnvalue_3 (`PrimitiveComponent.CreateDynamicMaterialInstance` (`/Game/Blueprints/Particle_Ball.Sphere` _returnvalue_2) 0 "/Game/Colors/ColorMaterial_Inst.ColorMaterial_Inst" "None"))
  (`MaterialInstanceDynamic.SetVectorParameterValue` _returnvalue_3 "Color" (`KismetMathLibrary.MakeColor` (`KismetMathLibrary.RandomFloatInRange` 0.0 255.0) (`KismetMathLibrary.RandomFloatInRange` 0.0 255.0) (`KismetMathLibrary.RandomFloatInRange` 0.0 255.0)))
  (`MaterialInstanceDynamic.SetScalarParameterValue` _returnvalue_3 "Intensity" (`KismetMathLibrary.RandomFloatInRange` 0.1 0.2))
  (set `/Game/Blueprints/Particle_Ball.ColorMaterial` _returnvalue_3 _returnvalue_2))

(event `ParticlesInit`
  (for _ (range (+ (`self.NumberOfParticles`) 1))
    (`self.AddParticle`)))

(event `self.ReceiveBeginPlay`
  (`self.ParticlesInit`)
  (`KismetSystemLibrary.K2_SetTimer` null "RunSimulation" 0.01 true)
  (`PlayerController.SetViewTargetWithBlend` (`GameplayStatics.GetPlayerControllerFromID` 0) self 0.0 "VTBlend_Linear" 0.0 false)
  (bind _returnvalue (`|CreateWidget` "/Game/Blueprints/SphereSimUI.SphereSimUI_C"))
  (`UserWidget.AddToViewport` _returnvalue 0)
  (`WidgetBlueprintLibrary.SetInputMode_GameAndUIEx` (`GameplayStatics.GetPlayerController` 0) _returnvalue "LockAlways"))

(event `self.ReceiveTick`
  (params (DeltaSeconds :type "Float (single-precision)")))

(fn `CalculateInverseSquaredForce`
  (params (P :type "Vector Structure") (Q :type "Vector Structure"))
  (returns (Force :type "Vector Structure"))
  (bind (_returnvalue_x _returnvalue_y _returnvalue_z) (`KismetMathLibrary.BreakVector` (- P Q)))
  (bind _returnvalue (`KismetMathLibrary.Sqrt` (+ (* _returnvalue_x _returnvalue_x) (* _returnvalue_y _returnvalue_y) (* _returnvalue_z _returnvalue_z))))
  (bind _returnvalue_2 (* _returnvalue _returnvalue _returnvalue))
  (return (* (/ (`KismetMathLibrary.MakeVector` _returnvalue_x _returnvalue_y _returnvalue_z) (`KismetMathLibrary.MakeVector` _returnvalue_2 _returnvalue_2 _returnvalue_2)) (`self.kr`))))

(fn `ContantPointEqSolver`
  (params (Location :type "Vector Structure") (Vecloty :type "Vector Structure") (SphereCenter :type "Vector Structure") (Mass :type "Float (double-precision)") (InvForce :type "Vector Structure"))
  (returns (NewLocation :type "Vector Structure") (NewVelocity :type "Vector Structure"))
  (bind _x (.x Location))
  (bind _y (.y Location))
  (bind _z (.z Location))
  (bind _x_2 (.x Vecloty))
  (bind _y_2 (.y Vecloty))
  (bind _z_2 (.z Vecloty))
  (bind _x_3 (.x SphereCenter))
  (bind _y_3 (.y SphereCenter))
  (bind _z_3 (.z SphereCenter))
  (bind _returnvalue (+ (`KismetMathLibrary.MultiplyMultiply_FloatFloat` _x_2 2.0) (`KismetMathLibrary.MultiplyMultiply_FloatFloat` _y_2 2.0) (`KismetMathLibrary.MultiplyMultiply_FloatFloat` _z_2 2.0)))
  (bind _returnvalue_2 (* _returnvalue 2.0))
  (bind _returnvalue_3 (+ (* (* (- _x _x_3) _x_2) 2.0) (* (* (- _y _y_3) _y_2) 2.0) (* (* (- _z _z_3) _z_2) 2.0)))
  (bind _returnvalue_4 (* _returnvalue_3 -1.0))
  (bind _returnvalue_5 (`KismetMathLibrary.Sqrt` (- (`KismetMathLibrary.MultiplyMultiply_FloatFloat` _returnvalue_3 2.0) (* 4.0 _returnvalue (- (+ (`KismetMathLibrary.MultiplyMultiply_FloatFloat` (- _x _x_3) 2.0) (`KismetMathLibrary.MultiplyMultiply_FloatFloat` (- _y _y_3) 2.0) (`KismetMathLibrary.MultiplyMultiply_FloatFloat` (- _z _z_3) 2.0)) (`KismetMathLibrary.MultiplyMultiply_FloatFloat` (`KismetMathLibrary.VSize` (- (`SceneComponent.K2_GetComponentLocation` (`self.SphereCenter`)) (`SceneComponent.K2_GetComponentLocation` (`self.SpherePoint`)))) 2.0))))))
  (bind _returnvalue_6 (/ (+ _returnvalue_4 _returnvalue_5) _returnvalue_2))
  (bind _returnvalue_7 (/ (- _returnvalue_4 _returnvalue_5) _returnvalue_2))
  (if (and (< _returnvalue_7 0.0) (< _returnvalue_6 0.0))
    (if (>= _returnvalue_6 _returnvalue_7)
      _
      (else
        (bind (_newlocation _newvelocity) (`self.Euler` Location Vecloty _returnvalue_7 Mass InvForce :!label _label))
        (return _newlocation _newvelocity)))
    (elif (>= _returnvalue_6 0.0)
      _
      (else
        (goto _label))))
  (bind (_newlocation_2 _newvelocity_2) (`self.Euler` Location Vecloty _returnvalue_6 Mass InvForce))
  (return _newlocation_2 _newvelocity_2))

(fn `DrawDebugDynamics`
  (params (Location :type "Vector Structure") (Velocity :type "Vector Structure") (Mass :type "Float (double-precision)") (InverseForce :type "Vector Structure"))
  (if (`self.Debug?`)
    (`KismetSystemLibrary.DrawDebugArrow` Location (+ Location (* InverseForce (100000.0 100000.0 100000.0))) 25.0 (struct :`R` 1.0 :`B` 0.018362 :`A` 1.0) 0.001 5.0)
    (`KismetSystemLibrary.DrawDebugArrow` Location (+ Location (* Velocity (100.0 100.0 100.0))) 25.0 (struct :`R` 0.974049 :`G` 1.0 :`A` 1.0) 0.001 5.0)))

(fn `Euler`
  (params (Location :type "Vector Structure") (Velocity :type "Vector Structure") (time :type "Float (double-precision)") (Mass :type "Float (double-precision)") (InverseForce :type "Vector Structure"))
  (returns (NewLocation :type "Vector Structure") (NewVelocity :type "Vector Structure"))
  (return (+ Location (* Velocity (`KismetMathLibrary.MakeVector` time time time))) (+ Velocity (* (/ InverseForce (`KismetMathLibrary.MakeVector` Mass Mass Mass)) (`KismetMathLibrary.MakeVector` time time time)))))

(fn `get_vector_float`
  (params (Vector1 :type "Vector Structure") (Vector2 :type "Vector Structure"))
  (returns (Result :type "Float (double-precision)"))
  (return (+ (* Vector1_X Vector2_X) (* Vector1_Y Vector2_Y) (* Vector1_Z Vector2_Z))))

(fn `RunSimulation`
  (bind _activeparticles (`self.ActiveParticles`))
  (bind _epsilon (`self.epsilon`))
  (`KismetArrayLibrary.Array_Clear` (`self.ForceSum`))
  (for _array_element _activeparticles
    (`self.SumInverseForces` _array_element))
  (for (_array_element_2 _array_index) _activeparticles
    (bind _location (`/Game/Blueprints/Particle_Ball.Location` _array_element_2))
    (bind _velocity (`/Game/Blueprints/Particle_Ball.Velocity` _array_element_2))
    (bind _mass (`/Game/Blueprints/Particle_Ball.Mass` _array_element_2))
    (bind _output (`|GetArrayItem` (`self.ForceSum`) _array_index))
    (`self.DrawDebugDynamics` _location _velocity _mass _output)
    (bind (_newlocation _newvelocity) (`self.Euler` _location _velocity (+ (`self.t`) (`self.t0`)) _mass _output))
    (if (`self.SphereCollisionDetection` _newlocation)
      (bind _newlocation_2 (`self.ContantPointEqSolver` _location _velocity (`SceneComponent.K2_GetComponentLocation` (`self.SphereCenter`)) _mass _output))
      (bind _output_get (set `/Game/Blueprints/Particle_Ball.Location` _newlocation_2 _array_element_2))
      (bind _returnvalue (`KismetMathLibrary.Normal` (- _newlocation (`SceneComponent.K2_GetComponentLocation` (`self.SphereCenter`)))))
      (set `/Game/Blueprints/Particle_Ball.Velocity` (+ (* (`KismetMathLibrary.MakeVector` _epsilon _epsilon _epsilon) _returnvalue) (- _velocity _returnvalue)) _array_element_2)
      (`SceneComponent.K2_SetWorldLocation` (`/Game/Blueprints/Particle_Ball.Sphere` _array_element_2) _output_get false false)
      (else
        (bind _output_get_2 (set `/Game/Blueprints/Particle_Ball.Location` _newlocation _array_element_2))
        (set `/Game/Blueprints/Particle_Ball.Velocity` _newvelocity _array_element_2)
        (`SceneComponent.K2_SetWorldLocation` (`/Game/Blueprints/Particle_Ball.Sphere` _array_element_2) _output_get_2 false false)))))

(fn `SphereCollisionDetection`
  (params (Location :type "Vector Structure"))
  (returns (`Collide?` :type Boolean))
  (bind _returnvalue (`SceneComponent.K2_GetComponentLocation` (`self.SphereCenter`)))
  (return (< (- (`KismetMathLibrary.VSize` (- _returnvalue (`SceneComponent.K2_GetComponentLocation` (`self.SpherePoint`)))) (`KismetMathLibrary.VSize` (- _returnvalue Location))) 0.0)))

(fn `SumInverseForces`
  (params (Particle :type "/Game/Blueprints/Particle_Ball Object Reference"))
  (locals (Sum :type "Vector Structure"))
  (for _array_element (`self.ActiveParticles`)
    (if (!= Particle _array_element)
      (bind _force (`self.CalculateInverseSquaredForce` (`SceneComponent.K2_GetComponentLocation` (`/Game/Blueprints/Particle_Ball.Sphere` Particle)) (`SceneComponent.K2_GetComponentLocation` (`/Game/Blueprints/Particle_Ball.Sphere` _array_element))))
      (set `local.Sum` (+ (`local.Sum`) _force))))
  (`KismetArrayLibrary.Array_Add` (`self.ForceSum`) (`local.Sum`))
  (return))

(fn `UserConstructionScript`)