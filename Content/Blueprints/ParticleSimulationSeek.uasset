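; Particle simulation actor that spawns colored spheres and seeker cubes by class in a box, demonstrating seek steering.
; BeginPlay shows SeekerUI, staggers spawning, switches the camera to a particle, then later destroys all particles.
; A looping timer, rather than Tick, runs Euler integration with gravity and mass, plus optional debug arrows.
; Seekers accelerate at MaxAcceleration toward the first other particle of their class.
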(event `AddParticle`
  (params (ParticleClass :type Integer) (ParticleMesh :type "StaticMesh Object Reference") (`Seeker?` :type Boolean))
  (bind _box (`self.Box`))
  (bind _returnvalue (`KismetMathLibrary.RandomPointInBoundingBox` (`SceneComponent.K2_GetComponentLocation` _box) (`BoxComponent.BoxExtent` _box)))
  (bind _returnvalue_2 (`|SpawnActorFromClass` "/Game/Blueprints/Particle_Hybrid.Particle_Hybrid_C" (`KismetMathLibrary.MakeTransform` _returnvalue (struct) (0.5 0.5 0.5)) "Undefined" "OverrideRootScale" null null))
  (`KismetArrayLibrary.Array_Add` (`self.ActiveParticles`) _returnvalue_2)
  (set `/Game/Blueprints/Particle_Hybrid.Class` ParticleClass _returnvalue_2)
  (set `/Game/Blueprints/Particle_Hybrid.Velocity` (`KismetMathLibrary.MakeVector` (`KismetMathLibrary.RandomFloatInRange` -1.0 1.0) (`KismetMathLibrary.RandomFloatInRange` -5.0 5.0) (`KismetMathLibrary.RandomFloatInRange` -10.0 5.0)) _returnvalue_2)
  (set `/Game/Blueprints/Particle_Hybrid.Mass` (`self.ParticleMass`) _returnvalue_2)
  (set `/Game/Blueprints/Particle_Hybrid.Location` _returnvalue _returnvalue_2)
  (bind _particle (`/Game/Blueprints/Particle_Hybrid.Particle` _returnvalue_2))
  (`StaticMeshComponent.SetStaticMesh` _particle ParticleMesh)
  (bind _returnvalue_3 (`PrimitiveComponent.CreateDynamicMaterialInstance` _particle 0 "/Game/Colors/ColorMaterial_Inst.ColorMaterial_Inst" "None"))
  (`MaterialInstanceDynamic.SetVectorParameterValue` _returnvalue_3 "Color" (`|GetArrayItem` (`self.ClassColors`) ParticleClass))
  (`MaterialInstanceDynamic.SetScalarParameterValue` _returnvalue_3 "Intensity" 10.0)
  (set `/Game/Blueprints/Particle_Hybrid.ColorMaterial` _returnvalue_3 _returnvalue_2)
  (set `/Game/Blueprints/Particle_Hybrid.Seeker?` `Seeker?` _returnvalue_2))

(event `self.ReceiveBeginPlay`
  (bind _returnvalue (`|CreateWidget` "/Game/Blueprints/SeekerUI.SeekerUI_C"))
  (`UserWidget.AddToViewport` _returnvalue 0)
  (`WidgetBlueprintLibrary.SetInputMode_GameAndUIEx` (`GameplayStatics.GetPlayerController` 0) _returnvalue)
  (`PlayerController.SetViewTargetWithBlend` (`GameplayStatics.GetPlayerControllerFromID` 0) self 0.0 "VTBlend_Linear" 0.0 false)
  (bind _returnvalue_2 (`KismetSystemLibrary.K2_SetTimer` null "RunSimulation" 0.03 true))
  (set `self.SimulationTimer` _returnvalue_2)
  (bind _result (`/Engine/EditorBlueprintResources/StandardMacros.DecrementInt` (`self.NumberOfClasses`))
    (:`  `
      (bind _index (`self.ForLoopWithDelay` 0 _result false 1.0)
        (:`LoopBody`
          (`self.AddParticle` _index "/Engine/BasicShapes/Sphere.Sphere"))
        (:`Completed`
          (`KismetSystemLibrary.Delay` 3.0)
          (bind _index_2 (`self.ForLoopWithDelay` 0 (`self.NumberOfClasses`) false 1.0)
            (:`LoopBody`
              (`self.AddParticle` _index_2 "/Engine/BasicShapes/Cube.Cube" true))
            (:`Completed`
              (`KismetSystemLibrary.Delay` 10.0)
              (bind _returnvalue_3 (`GameplayStatics.GetActorOfClass` "/Game/Blueprints/Particle_Hybrid.Particle_Hybrid_C"))
              (`PlayerController.SetViewTargetWithBlend` (`GameplayStatics.GetPlayerControllerFromID` 0) _returnvalue_3 0.0 "VTBlend_Linear" 0.0 false)
              (`KismetSystemLibrary.Delay` 30.0)
              (`KismetSystemLibrary.K2_ClearAndInvalidateTimerHandle` (`self.SimulationTimer`))
              (for _array_element (`self.ActiveParticles`)
                (`/Engine/EditorBlueprintResources/StandardMacros.IsValid` _array_element
                  (:`Is Valid`
                    (`self.K2_DestroyActor` _array_element))))
              (`KismetSystemLibrary.PrintString` "Simulation Ended"))))))))

(event `self.ReceiveTick`
  (params (DeltaSeconds :type "Float (single-precision)")))

(fn `DrawDebugDynamics`
  (params (Location :type "Vector Structure") (Velocity :type "Vector Structure") (Mass :type "Float (double-precision)") (Seek :type "Vector Structure"))
  (if (`self.Debug?`)
    (`KismetSystemLibrary.DrawDebugArrow` Location (* (+ Location (* Velocity (* (`self.gravity`) Mass))) (1.0 1.0 2.0)) 25.0 (struct :`R` 1.0 :`B` 0.018362 :`A` 1.0) 0.001 5.0)
    (`KismetSystemLibrary.DrawDebugArrow` Location (+ Location (* Velocity (100.0 100.0 100.0))) 25.0 (struct :`R` 0.974049 :`G` 1.0 :`A` 1.0) 0.001 5.0)
    (`KismetSystemLibrary.DrawDebugArrow` Location (+ Location (+ Velocity (* Seek (100.0 100.0 100.0)))) 25.0 (struct :`R` 0.09355 :`G` 0.817708 :`A` 1.0) 0.001 5.0)))

(fn `Euler`
  (params (Location :type "Vector Structure") (Velocity :type "Vector Structure") (time :type "Float (double-precision)") (Mass :type "Float (double-precision)") (SeekForce :type "Vector Structure"))
  (returns (NewLocation :type "Vector Structure") (NewVelocity :type "Vector Structure"))
  (bind _returnvalue (`KismetMathLibrary.MakeVector` Mass Mass Mass))
  (return (+ Location (* Velocity (`KismetMathLibrary.MakeVector` time time time))) (+ Velocity (* (/ (+ (* (`self.gravity`) _returnvalue) SeekForce) _returnvalue) (`KismetMathLibrary.MakeVector` time time time)))))

(fn `get_vector_float`
  (params (Vector1 :type "Vector Structure") (Vector2 :type "Vector Structure"))
  (returns (Result :type "Float (double-precision)"))
  (return (+ (* Vector1_X Vector2_X) (* Vector1_Y Vector2_Y) (* Vector1_Z Vector2_Z))))

(fn `LocateTarget`
  (params (SeekerClass :type Integer) (SeekerReference :type "Actor Object Reference"))
  (returns (TargetLocation :type "Vector Structure"))
  (for _array_element (`self.ActiveParticles`)
    (if (and (== (`/Game/Blueprints/Particle_Hybrid.Class` _array_element) SeekerClass) (!= SeekerReference _array_element))
      (return (`SceneComponent.K2_GetComponentLocation` (`/Game/Blueprints/Particle_Hybrid.Particle` _array_element))))))

(fn `RunSimulation`
  (bind _seekforcetemp (`self.SeekForceTemp`))
  (bind _activeparticles (`self.ActiveParticles`))
  (for (_array_element _array_index) _activeparticles
    (`/Engine/EditorBlueprintResources/StandardMacros.IsValid` _array_element
      (:`Is Valid`
        (if (`/Game/Blueprints/Particle_Hybrid.Seeker?` _array_element)
          (bind _location (`/Game/Blueprints/Particle_Hybrid.Location` _array_element))
          (set `self.SeekForceTemp` (`self.Seek` _location (`self.LocateTarget` (`/Game/Blueprints/Particle_Hybrid.Class` _array_element) _array_element)))
          (else
            (set `self.SeekForceTemp` (0.0 0.0 0.0))))
        (bind _velocity (`/Game/Blueprints/Particle_Hybrid.Velocity` _array_element))
        (bind _mass (`/Game/Blueprints/Particle_Hybrid.Mass` _array_element))
        (`self.DrawDebugDynamics` _location _velocity _mass _seekforcetemp)
        (bind (_newlocation _newvelocity) (`self.Euler` _location _velocity (+ (`self.t`) (`self.t0`)) _mass _seekforcetemp))
        (bind _output_get (set `/Game/Blueprints/Particle_Hybrid.Location` _newlocation _array_element))
        (set `/Game/Blueprints/Particle_Hybrid.Velocity` _newvelocity _array_element)
        (`SceneComponent.K2_SetWorldLocation` (`/Game/Blueprints/Particle_Hybrid.Particle` _array_element) _output_get false false))
      (:`Is Not Valid`
        (`KismetArrayLibrary.Array_Remove` _activeparticles _array_index)))))

(fn `Seek`
  (params (SeekerPosition :type "Vector Structure") (TargetPosition :type "Vector Structure"))
  (returns (A :type "Vector Structure"))
  (bind (_returnvalue_x _returnvalue_y _returnvalue_z) (`KismetMathLibrary.BreakVector` (- TargetPosition SeekerPosition)))
  (return (* (/ (`KismetMathLibrary.MakeVector` _returnvalue_x _returnvalue_y _returnvalue_z) (`KismetMathLibrary.Sqrt` (+ (* _returnvalue_x _returnvalue_x) (* _returnvalue_y _returnvalue_y) (* _returnvalue_z _returnvalue_z)))) (`self.maxAcceleration`))))

(fn `UserConstructionScript`)