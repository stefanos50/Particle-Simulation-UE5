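; SimulationController is an input Blueprint that switches between particle simulation demo levels.
; Number keys 1 to 8 each open a named level by name, covering particle, sphere, seek, rain, fire, bird flock and island scenes.
; The X key shows the mouse cursor, while BeginPlay, Tick and the construction script are left empty.
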(event `Key|X`
  (params (Key :type "Key Structure"))
  (:`Pressed`
    (set `self.bShowMouseCursor` true)))

(event `Key|One`
  (params (Key :type "Key Structure"))
  (:`Pressed`
    (`GameplayStatics.OpenLevel` "ParticleSimulation1")))

(event `Key|Two`
  (params (Key :type "Key Structure"))
  (:`Pressed`
    (`GameplayStatics.OpenLevel` "ParticleSimulation2_v2")))

(event `Key|Three`
  (params (Key :type "Key Structure"))
  (:`Pressed`
    (`GameplayStatics.OpenLevel` "ParticleSimulationSphere")))

(event `Key|Four`
  (params (Key :type "Key Structure"))
  (:`Pressed`
    (`GameplayStatics.OpenLevel` "ParticleSimulationSeek")))

(event `Key|Five`
  (params (Key :type "Key Structure"))
  (:`Pressed`
    (`GameplayStatics.OpenLevel` "ParticleSimulation_Rain")))

(event `Key|Six`
  (params (Key :type "Key Structure"))
  (:`Pressed`
    (`GameplayStatics.OpenLevel` "ParticleSimulation_Fire")))

(event `Key|Seven`
  (params (Key :type "Key Structure"))
  (:`Pressed`
    (`GameplayStatics.OpenLevel` "ParticleBirdFlock")))

(event `Key|Eight`
  (params (Key :type "Key Structure"))
  (:`Pressed`
    (`GameplayStatics.OpenLevel` "Island")))

(fn `UserConstructionScript`)